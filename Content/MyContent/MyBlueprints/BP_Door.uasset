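; BP_Door is a door that opens while any of its linked light targets is active.
; Each Tick it loops over the LightTargets array and sets DoorOpened if at least one target has IsActive set.
; When open, it hides the Cube mesh and disables its collision; otherwise the Cube is visible and solid again.
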(event `self.ReceiveTick`
  (params (DeltaSeconds :type "Float (single-precision)"))
  (bind _cube (`self.Cube`))
  (set `self.DoorOpened` false)
  (for _array_element (`self.LightTargets`)
    (if (`/Game/MyContent/MyBlueprints/BP_LightTarget.bIsActive` _array_element)
      (set `self.DoorOpened` true)))
  (if (`self.DoorOpened`)
    (`PrimitiveComponent.SetCollisionEnabled` _cube "NoCollision")
    (`SceneComponent.SetVisibility` _cube false false)
    (else
      (`PrimitiveComponent.SetCollisionEnabled` _cube "QueryAndPhysics")
      (`SceneComponent.SetVisibility` _cube true false))))

(fn `UserConstructionScript`)