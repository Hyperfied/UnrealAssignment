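; BP_LightEmitter is a rotatable light source that casts a colored beam to interactable actors.
; Any actor overlap sets InRange, which lets IA_Interact turn the Base by 90 degrees through player input enabled at BeginPlay.
; Every Tick it line-traces along the Arrow for BeamLength, drawn only as a debug line.
; Hit actors implementing BPI_LightInteractable receive BeamColor every frame they are hit.
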(event `self.ReceiveBeginPlay`
  (`self.EnableInput` (`GameplayStatics.GetPlayerController` 0)))

(event `self.ReceiveActorBeginOverlap`
  (params (OtherActor :type "Actor Object Reference"))
  (bind _output_get (set `self.InRange` true)))

(event `self.ReceiveActorEndOverlap`
  (params (OtherActor :type "Actor Object Reference"))
  (set `self.InRange` false))

(event `EnhancedInput|/Game/Input/Actions/IA_Interact`
  (params (ActionValue :type Boolean) (ElapsedSeconds :type "Float (double-precision)") (TriggeredSeconds :type "Float (double-precision)") (InputAction :type "InputAction Object Reference" :default "/Game/Input/Actions/IA_Interact.IA_Interact"))
  (:`Triggered`
    (if (stale `self.ReceiveActorBeginOverlap` _output_get)
      (`SceneComponent.K2_AddLocalRotation` (`self.Base`) (struct :`Yaw` 90.0) false false))))

(event `self.ReceiveTick`
  (params (DeltaSeconds :type "Float (single-precision)"))
  (bind _arrow (`self.Arrow`))
  (bind _returnvalue (`SceneComponent.K2_GetComponentLocation` _arrow))
  (bind (_outhit _returnvalue_2) (`KismetSystemLibrary.LineTraceSingle` :`Start` _returnvalue :`End` (+ _returnvalue (* (`self.BeamLength`) (`SceneComponent.GetForwardVector` _arrow))) :`TraceChannel` "TraceTypeQuery1" :`DrawDebugType` "ForOneFrame"))
  (if _returnvalue_2
    (bind (_bblockinghit _binitialoverlap _time _distance _location _impactpoint _normal _impactnormal _physmat _hitactor) (`GameplayStatics.BreakHitResult` _outhit))
    (`self.HandleHit` _location _hitactor)))

(event `HandleHit`
  (params (BeamHitLocation :type "Vector Structure") (HitActor :type "Actor Object Reference"))
  (if (`KismetSystemLibrary.DoesImplementInterface` HitActor "/Game/MyContent/MyBlueprints/BPI_LightInteractable.BPI_LightInteractable_C")
    (message `/Game/MyContent/MyBlueprints/BPI_LightInteractable.RecieveLight` HitActor (`self.BeamColor`) null)))

(fn `UserConstructionScript`)