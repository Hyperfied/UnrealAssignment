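; BP_Keypad is an interactable keypad puzzle that opens a linked door when its random three-digit code is solved.
; On BeginPlay it creates a W_Keypad widget, passes it the answer, gives one digit to each clue actor and prints the code.
; Interacting while overlapping toggles the keypad, blending to its camera, enabling the cursor and hiding the player.
; The widget holds a keypad reference for SolvedAnswer, which closes it and opens the door.
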(event `self.ReceiveBeginPlay`
  (bind _returnvalue (`KismetMathLibrary.RandomIntegerInRange` 0 9))
  (bind _widget (`self.Widget`))
  (bind _wkeypad (`self.WKeypad`))
  (bind _output_get (set `self.PlayerController` (`GameplayStatics.GetPlayerController` 0)))
  (`self.EnableInput` _output_get)
  (set `self.OldViewTarget` (`Controller.GetViewTarget` _output_get))
  (bind _returnvalue_2 (`|CreateWidget` "/Game/MyContent/Widgets/W_Keypad.W_Keypad_C" _output_get))
  (bind _output_get_2 (set `self.Widget` _returnvalue_2))
  (`WidgetComponent.SetWidget` _wkeypad _output_get_2)
  (`SceneComponent.SetVisibility` _wkeypad false false)
  (bind _output_get_3 (set `self.Digit1` _returnvalue))
  (bind _output_get_4 (set `self.Digit2` _returnvalue))
  (bind _output_get_5 (set `self.Digit3` _returnvalue))
  (`KismetSystemLibrary.DelayUntilNextTick`)
  (set `/Game/MyContent/Widgets/W_Keypad.Answer` (`|MakeArray` _output_get_3 _output_get_4 _output_get_5) _widget)
  (set `/Game/MyContent/Widgets/W_Keypad.Keypad` self _widget)
  (for (_array_element _array_index) (`self.Clues`)
    (switch `int` _array_index
      (:`0`
        (set `/Game/MyContent/Blueprints/BP_ClueTable.Digit` (`self.Digit1`) _array_element))
      (:`1`
        (set `/Game/MyContent/Blueprints/BP_ClueTable.Digit` (`self.Digit2`) _array_element))
      (:`2`
        (set `/Game/MyContent/Blueprints/BP_ClueTable.Digit` (`self.Digit3`) _array_element)))
    (set `/Game/MyContent/Blueprints/BP_ClueTable.Position` _array_index _array_element)
    (`/Game/MyContent/Blueprints/BP_ClueTable.SetClue` _array_element))
  (`KismetSystemLibrary.PrintString` (`KismetStringLibrary.BuildString_Int` (`KismetStringLibrary.BuildString_Int` (`KismetStringLibrary.BuildString_Int` "" "Code: " (`self.Digit1`)) "," (`self.Digit2`)) "," (`self.Digit3`))))

(event `self.ReceiveActorBeginOverlap`
  (params (OtherActor :type "Actor Object Reference"))
  (set `self.In Range` true))

(event `OpenWidget`
  (bind _playercontroller (`self.PlayerController`))
  (bind _playercontroller_2 (`self.PlayerController`))
  (bind _output_get (set `self.WidgetOpened` true))
  (`SceneComponent.SetVisibility` (`self.WKeypad`) _output_get false)
  (set `PlayerController.bShowMouseCursor` true _playercontroller)
  (set `PlayerController.bEnableClickEvents` true _playercontroller)
  (`WidgetBlueprintLibrary.SetInputMode_GameAndUIEx` _playercontroller_2 (`self.Widget`) "DoNotLock" false)
  (`PlayerController.SetViewTargetWithBlend` _playercontroller_2 (`self.Camera`) 0.5 "VTBlend_Linear" 0.0 false)
  (bind _asbp_third_person_player_controller (cast `/Game/ThirdPerson/Blueprints/BP_ThirdPersonPlayerController` _playercontroller_2))
  (`/Game/ThirdPerson/Blueprints/BP_ThirdPersonPlayerController.MakeInvis` _asbp_third_person_player_controller))

(event `self.ReceiveActorEndOverlap`
  (params (OtherActor :type "Actor Object Reference"))
  (set `self.In Range` false)
  (`self.CloseWidget`))

(event `CloseWidget`
  (bind _playercontroller (`self.PlayerController`))
  (bind _playercontroller_2 (`self.PlayerController`))
  (bind _output_get (set `self.WidgetOpened` false))
  (`SceneComponent.SetVisibility` (`self.WKeypad`) _output_get false)
  (set `PlayerController.bShowMouseCursor` false _playercontroller)
  (set `PlayerController.bEnableClickEvents` false _playercontroller)
  (`WidgetBlueprintLibrary.SetInputMode_GameOnly` _playercontroller_2)
  (`PlayerController.SetViewTargetWithBlend` _playercontroller_2 (`self.OldViewTarget`) 0.5 "VTBlend_Linear" 0.0 false)
  (bind _asbp_third_person_player_controller (cast `/Game/ThirdPerson/Blueprints/BP_ThirdPersonPlayerController` _playercontroller_2))
  (`/Game/ThirdPerson/Blueprints/BP_ThirdPersonPlayerController.Uninvis` _asbp_third_person_player_controller))

(event `EnhancedInput|/Game/Input/Actions/IA_Interact`
  (params (ActionValue :type Boolean) (ElapsedSeconds :type "Float (double-precision)") (TriggeredSeconds :type "Float (double-precision)") (InputAction :type "InputAction Object Reference" :default "/Game/Input/Actions/IA_Interact.IA_Interact"))
  (:`Triggered`
    (if (and (`self.In Range`) (not (`self.Solved`)))
      (if (`self.WidgetOpened`)
        (`self.CloseWidget`)
        (else
          (`self.OpenWidget`))))))

(event `SolvedAnswer`
  (`self.CloseWidget`)
  (`/Game/MyContent/Blueprints/BP_FireDoor.OpenDoor` (`self.Door`))
  (set `self.Solved` true))

(fn `UserConstructionScript`)