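; BP_LightTarget is a target that lights up in the color of a light beam that hits it and tracks whether it is active.
; BeginPlay gives the Cube a dynamic M_Target material instance.
; RecieveLight sets IsActive, drives emissive intensity and color from the beam, and starts a brief Deactivate timer.
; Repeated calls restart that timer, so the target returns to dark and inactive shortly after light stops arriving.
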(event `self.ReceiveBeginPlay`
  (`PrimitiveComponent.CreateDynamicMaterialInstance` (`self.Cube`) 0 "/Game/MyContent/Materials/m_Target.m_Target" "None"))

(event `/Game/MyContent/Blueprints/BPI_LightInteractable.RecieveLight`
  (params (BeamColor :type "Color Structure"))
  (bind (_r _g _b) (`KismetMathLibrary.BreakColor` (`KismetMathLibrary.Conv_ColorToLinearColor` BeamColor)))
  (set `self.bIsActive` true)
  (`MeshComponent.SetScalarParameterValueOnMaterials` (`self.Cube`) "EmissiveIntensity" 200.0)
  (`MeshComponent.SetVectorParameterValueOnMaterials` (`self.Cube`) "Color" (`KismetMathLibrary.MakeVector` _r _g _b))
  (`KismetSystemLibrary.K2_SetTimerDelegate` (delegate `/Game/MyContent/Blueprints/BPI_LightInteractable.Deactivate`) 0.1))

(event `/Game/MyContent/Blueprints/BPI_LightInteractable.Deactivate`
  (set `self.bIsActive` false)
  (`MeshComponent.SetScalarParameterValueOnMaterials` (`self.Cube`) "EmissiveIntensity" 0.0)
  (`MeshComponent.SetVectorParameterValueOnMaterials` (`self.Cube`) "Color" (`KismetMathLibrary.MakeVector` 0.026 0.026 0.026)))

(fn `UserConstructionScript`)