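; BP_ClueTable is an interactable clue actor that reveals a digit and its position through a W_Clue widget.
; On BeginPlay it enables player input, creates the widget, assigns it to the Clue component and copies in its Digit and Position.
; Any actor overlap sets an in-range flag that lets IA_Interact toggle the clue's visibility.
; Ending the overlap clears the flag and hides the clue.
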(event `self.ReceiveBeginPlay`
  (`self.EnableInput` (`GameplayStatics.GetPlayerController` 0))
  (bind _returnvalue (`|CreateWidget` "/Game/MyContent/Widgets/W_Clue.W_Clue_C"))
  (set `self.Widget` _returnvalue)
  (`WidgetComponent.SetWidget` (`self.Clue`) _returnvalue)
  (`self.SetClue`))

(event `self.ReceiveActorBeginOverlap`
  (params (OtherActor :type "Actor Object Reference"))
  (set `self.In Range` true))

(event `self.ReceiveActorEndOverlap`
  (params (OtherActor :type "Actor Object Reference"))
  (set `self.In Range` false)
  (`SceneComponent.SetVisibility` (`self.Clue`) false false :!label _label)
  (set `self.Visible` false))

(event `EnhancedInput|/Game/Input/Actions/IA_Interact`
  (params (ActionValue :type Boolean) (ElapsedSeconds :type "Float (double-precision)") (TriggeredSeconds :type "Float (double-precision)") (InputAction :type "InputAction Object Reference" :default "/Game/Input/Actions/IA_Interact.IA_Interact"))
  (:`Triggered`
    (if (`self.In Range`)
      (if (`self.Visible`)
        (goto _label)
        (else
          (`SceneComponent.SetVisibility` (`self.Clue`) true false)
          (set `self.Visible` true))))))

(event `SetClue`
  (bind _widget (`self.Widget`))
  (set `/Game/MyContent/Widgets/W_Clue.Digit` (`self.Digit`) _widget)
  (set `/Game/MyContent/Widgets/W_Clue.Position` (`self.Position`) _widget))

(fn `UserConstructionScript`)