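; BP_Door is a door that opens while any of its referenced LightTargets is active.
; BeginPlay gives the cube a dynamic material instance so its opacity can be animated.
; Tick polls the targets and acts only when the open state changes, toggling the cube's collision.
; The OpacityFadeOut timeline drives the Opacity parameter, playing from start on open and reversing from end on close.
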(event `self.ReceiveBeginPlay`
  (set `self.PrevDoorOpened` false)
  (bind _returnvalue (`PrimitiveComponent.CreateDynamicMaterialInstance` (`self.Cube`) 0 (`self.Source Material`) "None"))
  (bind _output_get (set `self.DynamicMat` _returnvalue))
  (`PrimitiveComponent.SetMaterial` (`self.Cube`) 0 _output_get))

(event `self.ReceiveTick`
  (params (DeltaSeconds :type "Float (single-precision)"))
  (bind _cube (`self.Cube`))
  (set `self.DoorOpened` false)
  (for _array_element (`self.LightTargets`)
    (if (`/Game/MyContent/Blueprints/BP_LightTarget.bIsActive` _array_element)
      (set `self.DoorOpened` true)))
  (if (!= (`self.PrevDoorOpened`) (`self.DoorOpened`))
    (set `self.PrevDoorOpened` (`self.DoorOpened`))
    (if (`self.DoorOpened`)
      (`PrimitiveComponent.SetCollisionEnabled` _cube "NoCollision")
      (bind (_direction _opacityfadeout) (`Timeline|OpacityFadeOut` :!via `PlayFromStart` :!label _label)
        (:`Update`
          (`MeshComponent.SetScalarParameterValueOnMaterials` (`self.Cube`) "Opacity" _opacityfadeout)))
      (else
        (`PrimitiveComponent.SetCollisionEnabled` _cube "QueryAndPhysics")
        (goto _label :!via `ReverseFromEnd`)))
    (else
      (set `self.PrevDoorOpened` (`self.DoorOpened`)))))

(fn `UserConstructionScript`)