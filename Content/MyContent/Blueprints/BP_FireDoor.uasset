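; BP_FireDoor is an interactable door that swings open around its yaw axis when the Interact input fires while an actor is overlapping it.
; It enables player input on BeginPlay and tracks range with overlap begin and end, without filtering which actor overlaps.
; A timeline drives the door's relative rotation, playing to open and reversing to close.
; A OneShot flag limits it to opening only; otherwise interaction toggles it.
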(event `self.ReceiveBeginPlay`
  (`self.EnableInput` (`GameplayStatics.GetPlayerController` 0)))

(event `EnhancedInput|/Game/Input/Actions/IA_Interact`
  (params (ActionValue :type Boolean) (ElapsedSeconds :type "Float (double-precision)") (TriggeredSeconds :type "Float (double-precision)") (InputAction :type "InputAction Object Reference" :default "/Game/Input/Actions/IA_Interact.IA_Interact"))
  (:`Triggered`
    (if (`self.In Range`)
      (if (`self.One Shot`)
        (`self.OpenDoor`)
        (elif (`self.Opened`)
          (`self.CloseDoor`)
          (else
            (`self.OpenDoor`)))))))

(event `self.ReceiveActorBeginOverlap`
  (params (OtherActor :type "Actor Object Reference"))
  (set `self.In Range` true))

(event `self.ReceiveActorEndOverlap`
  (params (OtherActor :type "Actor Object Reference"))
  (set `self.In Range` false))

(event `OpenDoor`
  (if (not (`self.Opened`))
    (set `self.Opened` true)
    (bind (_direction _rotation) (`Timeline|DoorOpen` :!label _label)
      (:`Update`
        (`SceneComponent.K2_SetRelativeRotation` (`self.Door`) (`KismetMathLibrary.MakeRotator` 0.0 0.0 _rotation) false false)))))

(event `CloseDoor`
  (if (`self.Opened`)
    (set `self.Opened` false)
    (goto _label :!via `Reverse`)))

(fn `UserConstructionScript`)