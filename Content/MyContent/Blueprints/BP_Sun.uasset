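; BP_Sun is an actor that bobs vertically around its starting position while its Sphere component spins.
; BeginPlay stores the start location, and each Tick offsets Z from it by a sine of game time, scaled by VerticalHeight and VerticalSpeed.
; Tick also adds local yaw to the Sphere, using OrbitSpeed scaled by delta time for a frame-rate-independent spin.
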(event `self.ReceiveBeginPlay`
  (set `self.StartPos` (`self.K2_GetActorLocation`)))

(event `self.ReceiveTick`
  (params (DeltaSeconds :type "Float (single-precision)"))
  (`self.K2_SetActorLocation` (+ (`self.StartPos`) (`KismetMathLibrary.MakeVector` 0.0 0.0 (* (`self.VerticalHeight`) (`KismetMathLibrary.DegSin` (* (`KismetSystemLibrary.GetGameTimeInSeconds`) (`self.VerticalSpeed`)))))))
  (`SceneComponent.K2_AddLocalRotation` (`self.Sphere`) (`KismetMathLibrary.MakeRotator` 0.0 0.0 (* DeltaSeconds (`self.OrbitSpeed`))) false false))

(fn `UserConstructionScript`)