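; BP_BirdView is an interactable actor that switches the player's view to its Camera, a bird's-eye view judging by the name.
; It enables input on itself and caches player controller 0's original view target at BeginPlay.
; While any actor overlap has set it in range, IA_Interact toggles between the two views with a short blend.
; Ending an overlap clears the range flag and restores the cached view.
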(event `self.ReceiveBeginPlay`
  (bind _output_get (set `self.PlayerCon` (`GameplayStatics.GetPlayerController` 0)))
  (`self.EnableInput` _output_get)
  (set `self.Old View Target` (`Controller.GetViewTarget` _output_get)))

(event `UseCamera`
  (set `self.In Use` true)
  (`PlayerController.SetViewTargetWithBlend` (`self.PlayerCon`) (`self.Camera`) 0.5 "VTBlend_Linear" 0.0 false))

(event `self.ReceiveActorBeginOverlap`
  (params (OtherActor :type "Actor Object Reference"))
  (set `self.In Range` true))

(event `CloseCamera`
  (set `self.In Use` false)
  (`PlayerController.SetViewTargetWithBlend` (`self.PlayerCon`) (`self.Old View Target`) 0.5 "VTBlend_Linear" 0.0 false))

(event `self.ReceiveActorEndOverlap`
  (params (OtherActor :type "Actor Object Reference"))
  (set `self.In Range` false)
  (`self.CloseCamera` :!label _label))

(event `EnhancedInput|/Game/Input/Actions/IA_Interact`
  (params (ActionValue :type Boolean) (ElapsedSeconds :type "Float (double-precision)") (TriggeredSeconds :type "Float (double-precision)") (InputAction :type "InputAction Object Reference" :default "/Game/Input/Actions/IA_Interact.IA_Interact"))
  (:`Triggered`
    (if (`self.In Range`)
      (if (`self.In Use`)
        (goto _label)
        (else
          (`self.UseCamera`))))))

(fn `UserConstructionScript`)